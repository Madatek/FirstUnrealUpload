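; Granny enemy character for the platform game, a child Blueprint that supplies the animation and hit areas for an area-type enemy.
; Its AttackAnimation event calls DoAttack on the ABP_AreaEnemy anim instance and stores the result as AnimationTime.
; Overlaps on the head, both arms and both feet all feed into ActorCollided, so each body part acts as a collision trigger.
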(event `self.AttackAnimation`
  (bind _attacktime (`/Game/PlatformGameUdemy/Art/Enemies/Area/ABP_AreaEnemy.DoAttack` (cast `/Game/PlatformGameUdemy/Art/Enemies/Area/ABP_AreaEnemy` (`SkeletalMeshComponent.GetAnimInstance` (`self.Mesh`)) :!pure true)))
  (set `self.AnimationTime` _attacktime))

(event `self.Head.OnComponentBeginOverlap`
  (params (OverlappedComponent :type "PrimitiveComponent Object Reference") (OtherActor :type "Actor Object Reference") (OtherComp :type "PrimitiveComponent Object Reference") (OtherBodyIndex :type Integer) (bFromSweep :type Boolean) (SweepResult :type "HitResult Structure (by ref)"))
  (`self.ActorCollided` OtherActor))

(event `self.LeftArm.OnComponentBeginOverlap`
  (params (OverlappedComponent :type "PrimitiveComponent Object Reference") (OtherActor :type "Actor Object Reference") (OtherComp :type "PrimitiveComponent Object Reference") (OtherBodyIndex :type Integer) (bFromSweep :type Boolean) (SweepResult :type "HitResult Structure (by ref)"))
  (`self.ActorCollided` OtherActor))

(event `self.RightArm.OnComponentBeginOverlap`
  (params (OverlappedComponent :type "PrimitiveComponent Object Reference") (OtherActor :type "Actor Object Reference") (OtherComp :type "PrimitiveComponent Object Reference") (OtherBodyIndex :type Integer) (bFromSweep :type Boolean) (SweepResult :type "HitResult Structure (by ref)"))
  (`self.ActorCollided` OtherActor))

(event `self.LeftFoot.OnComponentBeginOverlap`
  (params (OverlappedComponent :type "PrimitiveComponent Object Reference") (OtherActor :type "Actor Object Reference") (OtherComp :type "PrimitiveComponent Object Reference") (OtherBodyIndex :type Integer) (bFromSweep :type Boolean) (SweepResult :type "HitResult Structure (by ref)"))
  (`self.ActorCollided` OtherActor))

(event `self.RightFoot.OnComponentBeginOverlap`
  (params (OverlappedComponent :type "PrimitiveComponent Object Reference") (OtherActor :type "Actor Object Reference") (OtherComp :type "PrimitiveComponent Object Reference") (OtherBodyIndex :type Integer) (bFromSweep :type Boolean) (SweepResult :type "HitResult Structure (by ref)"))
  (`self.ActorCollided` OtherActor))

(fn `UserConstructionScript`
  (`parent.UserConstructionScript`))