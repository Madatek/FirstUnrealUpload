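; Groupie enemy Blueprint for a platform game, a radar-enemy variant that attacks with its right foot.
; Its AttackAnimation event calls DoDamage on the mesh's ABP_RadarEnemy anim instance and stores the result as AnimationTime.
; Overlaps on the RightFoot component pass the other actor to ActorCollided, which is defined outside this graph.
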(event `self.AttackAnimation`
  (bind _animationtime (`/Game/PlatformGameUdemy/Art/Enemies/Radar/ABP_RadarEnemy.DoDamage` (cast `/Game/PlatformGameUdemy/Art/Enemies/Radar/ABP_RadarEnemy` (`SkeletalMeshComponent.GetAnimInstance` (`self.Mesh`)) :!pure true)))
  (set `self.AnimationTime` _animationtime))

(event `self.RightFoot.OnComponentBeginOverlap`
  (params (OverlappedComponent :type "PrimitiveComponent Object Reference") (OtherActor :type "Actor Object Reference") (OtherComp :type "PrimitiveComponent Object Reference") (OtherBodyIndex :type Integer) (bFromSweep :type Boolean) (SweepResult :type "HitResult Structure (by ref)"))
  (`self.ActorCollided` OtherActor))

(fn `UserConstructionScript`
  (`parent.UserConstructionScript`))