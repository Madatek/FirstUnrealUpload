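; Green Dragon player character Blueprint that adds sideways dodges and a held dash on top of its parent class.
; BeginPlay binds the dodge and melee attack 1 events, with press and release doubling and restoring walk speed.
; Dodges, guarded by IsDodging, play animations and launch the character sideways, angled up from ground or down in air.
; Also defines helpers for character-state branching and timed looping timers, unused in its event graph.
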(event `DodgeRight`
  (if (not (`self.bIsDodging`))
    (set `self.bIsDodging` true)
    (if (`NavMovementComponent.IsFalling` (`self.CharacterMovement`))
      (`self.AnimationDodgeRight`)
      (`self.LaunchCharacter` (+ (* (`self.GetActorUpVector`) -150.0) (* (`self.GetActorRightVector`) 1000.0)) true true)
      (else
        (`self.AnimationDodgeRight`)
        (`self.LaunchCharacter` (+ (* (`self.GetActorUpVector`) 150.0) (* (`self.GetActorRightVector`) 1000.0)) true true)))))

(event `self.ReceiveBeginPlay`
  (`parent.ReceiveBeginPlay`)
  (add `self.OnDodgeLeft` (delegate `DodgeLeft`))
  (add `self.OnDodgeRight` (delegate `DodgeRight`))
  (add `self.OnMeleeAttack1Pressed` (delegate `StartDash`))
  (add `self.OnMeleeAttack1Released` (delegate `EndDash`)))

(event `DodgeLeft`
  (if (not (`self.bIsDodging`))
    (set `self.bIsDodging` true)
    (if (`NavMovementComponent.IsFalling` (`self.CharacterMovement`))
      (`self.AnimationDodgeLeft`)
      (`self.LaunchCharacter` (+ (* (`self.GetActorUpVector`) -150.0) (* (`self.GetActorRightVector`) -1000.0)) true true)
      (else
        (`self.AnimationDodgeLeft`)
        (`self.LaunchCharacter` (+ (* (`self.GetActorUpVector`) 150.0) (* (`self.GetActorRightVector`) -1000.0)) true true)))))

(event `EndDash`
  (set `CharacterMovementComponent.MaxWalkSpeed` 600.0 (`self.CharacterMovement`)))

(event `StartDash` :!signature `self.OnMeleeAttack1Pressed`
  (params (bPressed :type Boolean))
  (set `CharacterMovementComponent.MaxWalkSpeed` 1200.0 (`self.CharacterMovement`)))

(fn `UserConstructionScript`
  (`parent.UserConstructionScript`))