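; Donut point collectable for a platform game, a child Blueprint that varies its look at random.
; On BeginPlay it runs the parent logic, then creates a dynamic material instance on the collectable mesh.
; It sets that material's donut texture parameter to a randomly picked chocolate, caramel or red texture.
; The file adds no other active logic.
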(event `self.ReceiveBeginPlay`
  (`parent.ReceiveBeginPlay`)
  (bind _returnvalue (`PrimitiveComponent.CreateDynamicMaterialInstance` (`self.CollectableMesh`) 0 null "None"))
  (`MaterialInstanceDynamic.SetTextureParameterValue` _returnvalue "DonutTexture" (select `int` (`KismetMathLibrary.RandomIntegerInRange` 0 2) :`0` "/Game/PlatformGameUdemy/Art/Collectables/Point/T_ChocoDonut_D.T_ChocoDonut_D" :`1` "/Game/PlatformGameUdemy/Art/Collectables/Point/Texture_Variations/T_CaramelDonut_D.T_CaramelDonut_D" :`2` "/Game/PlatformGameUdemy/Art/Collectables/Point/Texture_Variations/T_RedDonut_D.T_RedDonut_D" :!type "Texture Object Reference")))

(fn `UserConstructionScript`
  (`parent.UserConstructionScript`))