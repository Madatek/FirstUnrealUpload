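; BP_BB_BE_TNT is a timed TNT box for a platformer, built on a parent box Blueprint.
; The first UpHit starts a one-shot BombTime timer, enables Tick, reveals TextTimer and calls the parent hit logic.
; Tick shows the remaining timer time as a rounded countdown on TextTimer.
; When the timer ends it calls Destroy, whose override runs Explosion before the parent's destroy logic.
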(event `self.ReceiveTick`
  (params (DeltaSeconds :type "Float (single-precision)"))
  (`parent.ReceiveTick` DeltaSeconds)
  (`TextRenderComponent.K2_SetText` (`self.TextTimer`) (`KismetTextLibrary.Conv_DoubleToText` (`KismetSystemLibrary.K2_GetTimerRemainingTimeHandle` (`self.TimerHandle`)) "HalfToEven" false true 1 324 0 0)))

(event `self.UpHit`
  (`/Engine/EditorBlueprintResources/StandardMacros.DoOnce` false
    (:`Completed`
      (bind _returnvalue (`KismetSystemLibrary.K2_SetTimerDelegate` (delegate `TimerEnd`) (`self.BombTime`)))
      (set `self.TimerHandle` _returnvalue)
      (`self.SetActorTickEnabled` true)
      (`SceneComponent.SetHiddenInGame` (`self.TextTimer`) false false)
      (`parent.UpHit`))))

(event `TimerEnd`
  (`self.Destroy` null))

(event `self.Destroy`
  (params (DamageCauser :type "Actor Object Reference"))
  (`self.Explosion`)
  (`parent.Destroy` null))

(fn `UserConstructionScript`
  (`parent.UserConstructionScript`))