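; Base Blueprint for explosive boxes in a platform game, providing a shared Explosion event that damages its surroundings.
; Explosion applies full radial damage with no falloff around the actor's location, out to ExplosionRadius.
; When Debug is enabled, it also draws a sphere showing the radius and spawns the explosion emitter, so the particle effect depends on that flag.
; The construction script only calls its parent.
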(event `Explosion`
  (bind _returnvalue (`self.K2_GetActorLocation`))
  ;[1 1 1] Explosion
  (`GameplayStatics.ApplyRadialDamage` :`BaseDamage` 100.0 :`Origin` _returnvalue :`DamageRadius` (`self.ExplosionRadius`) :`DamageCauser` self :`InstigatedByController` null :`bDoFullDamage` true)
  (if (`self.bDebug`)
    (`KismetSystemLibrary.DrawDebugSphere` _returnvalue (`self.ExplosionRadius`) 12 (struct :`R` 1.0 :`B` 0.044384 :`A` 1.0) 0.2 0.1)
    (`GameplayStatics.SpawnEmitterAtLocation` (`self.EmitterToSpawn`) _returnvalue)))

(fn `UserConstructionScript`
  (`parent.UserConstructionScript`))