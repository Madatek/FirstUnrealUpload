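; Base breakable box for a platformer, typed as Simple, Armored (explosive damage only) or Indestructible.
; Hit side picks an event: top hits launch the player and damage the box, bottom hits damage it, side handling is empty.
; Destruction spawns collectables, auto-collecting some, and reports counted boxes to BP_PlatformGameMode.
; The construction script applies type texture, debug color and label, while BoxActivation toggles color alpha, label and collision.
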(event `self.ReceiveAnyDamage`
  (params (Damage :type "Float (single-precision)") (DamageType :type "DamageType Object Reference") (InstigatedBy :type "Controller Object Reference") (DamageCauser :type "Actor Object Reference"))
  ;[1 1 1] Damage
  (switch `/Game/PlatformGameUdemy/Core/Interactables/Boxes/EBoxType` (`self.BoxType`)
    (:`NewEnumerator0`
      _)
    (:`NewEnumerator1`
      (cast `/Game/PlatformGameUdemy/Core/GameFramework/DamageTypes/BP_ExplosiveDamage` DamageType)))
  (bind _output_get (set `self.HealthPoints` (- (`self.HealthPoints`) Damage)))
  (if (<= _output_get 0.0)
    (`self.Destroy` DamageCauser)))

(event `self.ReceiveBeginPlay`
  ;[1 1 1] On spawn
  (bind _output_get (set `self.ReferenceGameMode` (cast `/Game/PlatformGameUdemy/Core/GameFramework/BP_PlatformGameMode` (`GameplayStatics.GetGameMode`) :!pure true)))
  (if (`self.bBoxToCount`)
    (`/Game/PlatformGameUdemy/Core/GameFramework/BP_PlatformGameMode.IncrementBoxTotal` _output_get)))

(event `self.ReceiveHit`
  (params (MyComp :type "PrimitiveComponent Object Reference") (Other :type "Actor Object Reference") (OtherComp :type "PrimitiveComponent Object Reference") (bSelfMoved :type Boolean) (HitLocation :type "Vector Structure") (HitNormal :type "Vector Structure") (NormalImpulse :type "Vector Structure") (Hit :type "HitResult Structure (by ref)"))
  ;[1 1 1] Hit related
  (set `self.HitInstigator` Other)
  (`KismetSystemLibrary.Delay` 0.1)
  (switch `/Game/PlatformGameUdemy/Core/Interactables/Common/EHitSide` (`/Game/PlatformGameUdemy/Core/Utility/BP_FL_Utility.CheckHitSide` HitNormal 0.1)
    (:`NewEnumerator0`
      (`self.OtherFaceHit` :!label _label)
      (set `self.HitInstigator` null))
    (:`NewEnumerator1`
      (goto _label))
    (:`NewEnumerator2`
      (goto _label))
    (:`NewEnumerator3`
      (goto _label))
    (:`NewEnumerator4`
      (`self.UpHit`)
      (`KismetSystemLibrary.Delay` 0.3)
      (bind _output_get (set `self.HitInstigator` null))
      (bind _asbp_base_player (cast `/Game/PlatformGameUdemy/Core/Characters/Player/BP_BasePlayer` _output_get))
      (set `/Game/PlatformGameUdemy/Core/Characters/Player/BP_BasePlayer.CanBeLaunched` false _asbp_base_player))
    (:`NewEnumerator5`
      (`self.DownHit`)
      (set `self.HitInstigator` null))))

(event `Destroy`
  (params (DamageCauser :type "Actor Object Reference"))
  ;[1 1 1] Destroyed
  (if (`self.bBoxToCount`)
    (`/Game/PlatformGameUdemy/Core/GameFramework/BP_PlatformGameMode.BoxBroken` (`self.ReferenceGameMode`)))
  (`self.SpawnCollectables` (`self.NumberOfCollectablesToSpawn`) (`self.Collect at Spawn`))
  (`self.K2_DestroyActor`))

(event `DownHit`
  ;[1 1 1] Hit related
  (`self.DamageAtJump`))

(event `OtherFaceHit`
  ;[1 1 1] Hit related
)

(event `BoxActivation`
  (params (Activate :type Boolean))
  ;[1 1 1] Activated by trigger
  (`MaterialInstanceDynamic.SetVectorParameterValue` (`self.DebugMaterial`) "BoxColor" (`self.GetDebugColorWithOrWithoutAlpha` Activate))
  (`SceneComponent.SetHiddenInGame` (`self.TextRender`) (not Activate) false)
  (`self.SetActorEnableCollision` Activate))

(event `UpHit`
  ;[1 1 1] Hit related
  (bind _asbp_base_player (cast `/Game/PlatformGameUdemy/Core/Characters/Player/BP_BasePlayer` (`self.HitInstigator`))
    (:`then`
      (set `/Game/PlatformGameUdemy/Core/Characters/Player/BP_BasePlayer.CanBeLaunched` true _asbp_base_player)
      (if true
        (message `/Game/PlatformGameUdemy/Core/Interactables/Common/Bp_Interactables.Launch Actor` (`self.HitInstigator`) (`self.LaunchActorSpeed`))
        (`self.DamageAtJump`)))
    (:`CastFailed`
      (set `self.HitInstigator` null))))

(fn `DamageAtJump`
  (`GameplayStatics.ApplyDamage` self (`self.JumpDamage`) null (`self.HitInstigator`)))

(fn `DummyBoxToCountGameManager`)

(fn `GetDebugColorWithOrWithoutAlpha`
  (params (WithAlpha :type Boolean))
  (returns (OutColor :type "LinearColor Structure"))
  (bind (_debugboxcolor_r _debugboxcolor_g _debugboxcolor_b _debugboxcolor_a) (break `LinearColor` (`self.DebugBoxColor`)))
  (return (select `bool` WithAlpha :`false` (make `LinearColor` _debugboxcolor_r _debugboxcolor_g _debugboxcolor_b) :`true` (make `LinearColor` _debugboxcolor_r _debugboxcolor_g _debugboxcolor_b _debugboxcolor_a) :!type "LinearColor Structure")))

(fn `SpawnCollectables`
  (params (NumberOfCollectables :type Integer) (bCollectAtSpawn :type Boolean))
  (bind _returnvalue (`self.K2_GetActorLocation`))
  (set `self.Collect at Spawn` bCollectAtSpawn)
  (for _ (range NumberOfCollectables)
    (bind _returnvalue_2 (`|SpawnActorFromClass` (`self.CollectablesType`) (`KismetMathLibrary.MakeTransform` (select `bool` (> NumberOfCollectables 1) :`false` _returnvalue :`true` (`KismetMathLibrary.RandomPointInBoundingBox` _returnvalue (50.0 50.0 0.0)))) "Undefined" "OverrideRootScale" null null))
    (if (`self.Collect at Spawn`)
      (bind _asbp_base_collectable (cast `/Game/PlatformGameUdemy/Core/Interactables/Collectables/BP_BaseCollectable` _returnvalue_2 :!pure true))
      (`/Game/PlatformGameUdemy/Core/Interactables/Collectables/BP_BaseCollectable.Collected` _asbp_base_collectable)
      (else
        (bind (_asbp_bc_target _bsuccess) (cast `/Game/PlatformGameUdemy/Core/Interactables/Collectables/BP_BC_Target` _asbp_base_collectable :!pure true))
        (if _bsuccess
          (`/Game/PlatformGameUdemy/Core/Interactables/Collectables/BP_BaseCollectable.Collected` _asbp_bc_target)
          (else
            (bind (_asbp_bc_life _bsuccess_2) (cast `/Game/PlatformGameUdemy/Core/Interactables/Collectables/BP_BC_Life` _asbp_base_collectable :!pure true))
            (if _bsuccess_2
              (`/Game/PlatformGameUdemy/Core/Interactables/Collectables/BP_BaseCollectable.Collected` _asbp_bc_life)))))))
  (return))

(fn `UserConstructionScript`
  (`|ExecutionSequence`
    (:`then_0`
      (bind _returnvalue (`PrimitiveComponent.CreateDynamicMaterialInstance` (`self.BoxMesh`) 0 null "None"))
      (bind _output_get (set `self.DebugMaterial` _returnvalue))
      (`MaterialInstanceDynamic.SetVectorParameterValue` (`self.DebugMaterial`) "BoxColor" (`self.DebugBoxColor`))
      (`MaterialInstanceDynamic.SetVectorParameterValue` _output_get "BoxColor" (`self.DebugBoxColor`))
      (`TextRenderComponent.K2_SetText` (`self.TextRender`) (`self.DebugBoxName`))
      (`MaterialInstanceDynamic.SetTextureParameterValue` _output_get "BoxTexture" (select `/Game/PlatformGameUdemy/Core/Interactables/Boxes/EBoxType` (`self.BoxType`) :`NewEnumerator0` "/Game/PlatformGameUdemy/Art/Box/T_NormalCorners.T_NormalCorners" :`NewEnumerator1` "/Game/PlatformGameUdemy/Art/Box/T_ArmoredCorners.T_ArmoredCorners" :`NewEnumerator2` "/Game/PlatformGameUdemy/Art/Box/T_IndestructibleCorners.T_IndestructibleCorners" :!type "Texture Object Reference")))
    (:`then_1`
      (`self.BoxActivation` (`self.bIsActive`))
      (if (`|EnumEquality` (`self.BoxType`) "NewEnumerator2")
        (set `self.bBoxToCount` false)))))