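; BP_BaseWarp is a base interactable warp for the platform game that players can use once it has been activated.
; WarpActivation, usually triggered by collecting a target, sets IsActive and swaps the warp particle effect onto WarpEffect.
; While active, a Player-tagged actor overlapping InteractionArea calls WarpInteracted, which here only prints a debug message.
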(event `self.InteractionArea.OnComponentBeginOverlap`
  (params (OverlappedComponent :type "PrimitiveComponent Object Reference") (OtherActor :type "Actor Object Reference") (OtherComp :type "PrimitiveComponent Object Reference") (OtherBodyIndex :type Integer) (bFromSweep :type Boolean) (SweepResult :type "HitResult Structure (by ref)"))
  ;[1 1 1] Begin overlap - if active, interact
  (if (and (`self.ActorHasTag` OtherActor "Player") (`self.bIsActive`))
    (`self.WarpInteracted`)))

(event `WarpInteracted`
  ;[1 1 1] When warp is interacted - debug only
  (`KismetSystemLibrary.PrintString` "Warp Interacted By Player"))

(event `WarpActivation`
  ;[1 1 1] Called on activation - usally when collecting the target
  (set `self.bIsActive` true)
  (`ParticleSystemComponent.SetTemplate` (`self.WarpEffect`) (`self.WarpParticleEffect`))
  (`KismetSystemLibrary.PrintString` "Warp Activated"))

(fn `UserConstructionScript`)