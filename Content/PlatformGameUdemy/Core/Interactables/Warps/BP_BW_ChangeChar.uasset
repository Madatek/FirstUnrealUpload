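; Warp interactable Blueprint that switches the player's character when interacted with.
; WarpInteracted clears IsActive and delegates the swap to the game mode's SwapPlayer, then runs a five-second delay with nothing after it.
; Helper functions fetch the controller and pawn, toggle between BigVegas and GreenDragon classes, and spawn a pawn above the warp, but the event calls none of them.
; DisableController is an empty stub.
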(event `self.WarpInteracted`
  (set `self.bIsActive` false)
  (`/Game/PlatformGameUdemy/Core/GameFramework/BP_PlatformGameMode.SwapPlayer` (cast `/Game/PlatformGameUdemy/Core/GameFramework/BP_PlatformGameMode` (`GameplayStatics.GetGameMode`) :!pure true) false)
  (`KismetSystemLibrary.Delay` 5.0))

(fn `DisableController`)

(fn `GetNextClass`
  (returns (NextSpawnedClass :type "Actor Class Reference"))
  (if (== (`GameplayStatics.GetObjectClass` (`self.CurrentPawn`)) "/Game/PlatformGameUdemy/Characters/Player/BP_BP_BigVegas.BP_BP_BigVegas_C")
    (set `self.NextSpawnedClass` "/Game/PlatformGameUdemy/Characters/Player/BP_BP_GreenDragon.BP_BP_GreenDragon_C")
    (else
      (set `self.NextSpawnedClass` "/Game/PlatformGameUdemy/Characters/Player/BP_BP_BigVegas.BP_BP_BigVegas_C")))
  (return (`self.NextSpawnedClass`)))

(fn `GetPawnAndController`
  (returns (PlayerController :type "/Game/PlatformGameUdemy/Core/Characters/Player/BP_PlatfromPlayerController Object Reference") (Pawn :type "Pawn Object Reference"))
  (bind _output_get (set `self.BPPlayerController` (cast `/Game/PlatformGameUdemy/Core/Characters/Player/BP_PlatfromPlayerController` (`GameplayStatics.GetPlayerController` 0) :!pure true)))
  (return _output_get (`Controller.K2_GetPawn` _output_get)))

(fn `SpawnNewPawn`
  (params (Class :type "Actor Class Reference"))
  (returns (ReturnValue :type "Actor Object Reference"))
  (bind _returnvalue (`|SpawnActorFromClass` Class (`KismetMathLibrary.MakeTransform` (+ (`self.K2_GetActorLocation`) (0.0 0.0 100.0))) "Undefined" "OverrideRootScale" null null))
  (return _returnvalue))

(fn `UserConstructionScript`
  (`parent.UserConstructionScript`))