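; Win warp actor for the platform game that ends the level in a victory once the player uses it.
; On BeginPlay it binds to the game mode's target-collected event, which triggers the inherited warp activation.
; When the warp is interacted with, it calls WinGame on BP_PlatformGameMode.
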(event `self.ReceiveBeginPlay`
  ;[1 1 1] On spawn
  (`parent.ReceiveBeginPlay`)
  (bind _asbp_platform_game_mode (cast `/Game/PlatformGameUdemy/Core/GameFramework/BP_PlatformGameMode` (`GameplayStatics.GetGameMode`)))
  (add `/Game/PlatformGameUdemy/Core/GameFramework/BP_PlatformGameMode.OnTargetCollected` _asbp_platform_game_mode (delegate `PortalActivation`)))

(event `PortalActivation`
  ;[1 1 1] On spawn
  (`self.WarpActivation`))

(event `self.WarpInteracted`
  ;[1 1 1] Call win game on game mode
  (bind _asbp_platform_game_mode (cast `/Game/PlatformGameUdemy/Core/GameFramework/BP_PlatformGameMode` (`GameplayStatics.GetGameMode`)))
  (`/Game/PlatformGameUdemy/Core/GameFramework/BP_PlatformGameMode.WinGame` _asbp_platform_game_mode))

(fn `UserConstructionScript`
  (`parent.UserConstructionScript`))