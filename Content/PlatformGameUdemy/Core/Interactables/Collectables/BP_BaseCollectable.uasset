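; Base collectable actor that reports its type to BP_PlatformGameMode and destroys itself when the player overlaps it.
; A timeline animates its height on spawn, enabling collision when finished, or immediately if CollectAtSpawn is set.
; The first damage launches it horizontally away from the causer with physics and a short lifespan; non-player overlaps during launch only print debug text.
; The construction script tints a dynamic material with DebugColor.
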(event `self.ReceiveBeginPlay`
  (if (`self.bCollectAtSpawn`)
    (`self.ActivateCollectableCollision`))
  (set `self.SpawnLocation` (`self.K2_GetActorLocation`))
  (bind (_direction _animationz) (`Timeline|SpawnAnimation`)
    (:`Update`
      (`self.K2_SetActorRelativeLocation` (+ (`self.SpawnLocation`) (`KismetMathLibrary.MakeVector` 0.0 0.0 _animationz))))
    (:`Finished`
      (`self.SpawnAnimationFinished`))))

(event `SpawnAnimationFinished`
  (`self.ActivateCollectableCollision`))

(event `self.ReceiveActorBeginOverlap`
  (params (OtherActor :type "Actor Object Reference"))
  (`/Game/PlatformGameUdemy/Core/Utility/BPML_Utility.ActorIsPlayer` OtherActor
    (:`IsPlayer`
      (`self.Collected`)
      (`self.K2_DestroyActor`))
    (:`IsNotPlayer`
      (if (`self.bLaunched`)
        (`self.OverlapDuringLaunch` OtherActor)))))

(event `Collected`
  (`/Game/PlatformGameUdemy/Core/GameFramework/BP_PlatformGameMode.AddCollectable` (cast `/Game/PlatformGameUdemy/Core/GameFramework/BP_PlatformGameMode` (`GameplayStatics.GetGameMode`) :!pure true) (`self.CollectableType`)))

(event `OverlapDuringLaunch`
  (params (OtherActor :type "Actor Object Reference"))
  (`KismetSystemLibrary.PrintString` (`KismetStringLibrary.Concat_StrStr` (`KismetSystemLibrary.GetDisplayName` OtherActor) "OvcrlapDuringLaunch")))

(event `self.ReceiveAnyDamage`
  (params (Damage :type "Float (single-precision)") (DamageType :type "DamageType Object Reference") (InstigatedBy :type "Controller Object Reference") (DamageCauser :type "Actor Object Reference"))
  (bind _collectablemesh (`self.CollectableMesh`))
  (bind (_returnvalue_x _returnvalue_y) (`KismetMathLibrary.BreakVector` (* (- (`self.K2_GetActorLocation`) (`self.K2_GetActorLocation` DamageCauser)) 6000.0)))
  (`/Engine/EditorBlueprintResources/StandardMacros.DoOnce` false
    (:`Completed`
      (`PrimitiveComponent.SetSimulatePhysics` _collectablemesh true)
      (`PrimitiveComponent.AddForce` _collectablemesh (`KismetMathLibrary.MakeVector` _returnvalue_x _returnvalue_y) "None" true)
      (set `self.bLaunched` true)
      (`self.SetLifeSpan` 3.0))))

(fn `ActivateCollectableCollision`
  (`PrimitiveComponent.SetCollisionEnabled` (`self.CollectableMesh`) "QueryAndPhysics"))

(fn `PLACEHOLDER_AddCollectable`
  (params (ReferenceGameMode :type "GameMode Object Reference") (CollectableType :type "/Game/PlatformGameUdemy/Core/Interactables/Collectables/ECollectableType Enum" :default "NewEnumerator0"))
  (`KismetSystemLibrary.PrintString` (`|GetEnumeratorNameAsString` CollectableType)))

(fn `UserConstructionScript`
  (bind _returnvalue (`PrimitiveComponent.CreateDynamicMaterialInstance` (`self.CollectableMesh`) 0 null "None"))
  (bind _output_get (set `self.MaterialInstanceRef` _returnvalue))
  (`MaterialInstanceDynamic.SetVectorParameterValue` (`self.MaterialInstanceRef`) "CollectableColor" (`self.DebugColor`))
  (`MaterialInstanceDynamic.SetVectorParameterValue` _output_get "CollectableColor" (`self.DebugColor`)))