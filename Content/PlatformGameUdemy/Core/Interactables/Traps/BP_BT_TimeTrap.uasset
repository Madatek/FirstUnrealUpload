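; Base timed trap Blueprint for the platformer that fires an empty DoAction event on a timer, apparently left for child traps to implement.
; BeginPlay starts the timer through TimerManager, which can also clear it, and optionally triggers DoAction immediately.
; The interval is AnimationDelay plus AnimationTimer, both clamped in the construction script, with optional looping.
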(event `self.ReceiveBeginPlay`
  (`parent.ReceiveBeginPlay`)
  (`self.Timer Manager` false)
  (if (`self.bTimerImmediatelyStarts`)
    (`self.DoAction`)))

(event `DoAction`)

(fn `Timer Manager`
  (params (bStop :type Boolean))
  (if bStop
    (`KismetSystemLibrary.K2_ClearAndInvalidateTimerHandle` (`self.TrapTimer`))
    (else
      (bind _returnvalue (`KismetSystemLibrary.K2_SetTimer` null "DoAction" (+ (`self.AnimationDelay`) (`self.AnimationTimer`)) (`self.bLoopTimer`)))
      (set `self.TrapTimer` _returnvalue)))
  (return))

(fn `UserConstructionScript`
  (`parent.UserConstructionScript`)
  (set `self.AnimationTimer` (`KismetMathLibrary.FClamp` (`self.AnimationTimer`) 1.5 4.5))
  (set `self.AnimationDelay` (`KismetMathLibrary.FClamp` (`self.AnimationDelay`))))