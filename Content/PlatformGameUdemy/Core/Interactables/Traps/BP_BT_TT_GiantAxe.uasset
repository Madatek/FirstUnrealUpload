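; A giant axe trap that swings and damages the player on contact.
; When DoAction fires, a timeline drives the actor's pitch while keeping its roll and yaw, with play rate scaled so the swing matches AnimationTimer.
; Overlaps on the axe collision are filtered to the player and passed to DoDamage.
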(event `self.AxeCollision.OnComponentBeginOverlap`
  (params (OverlappedComponent :type "PrimitiveComponent Object Reference") (OtherActor :type "Actor Object Reference") (OtherComp :type "PrimitiveComponent Object Reference") (OtherBodyIndex :type Integer) (bFromSweep :type Boolean) (SweepResult :type "HitResult Structure (by ref)"))
  ;[1 1 1] Axe hit
  (`/Game/PlatformGameUdemy/Core/Utility/BPML_Utility.ActorIsPlayer` OtherActor
    (:`IsPlayer`
      (`self.DoDamage` OtherActor))))

(event `self.DoAction`
  (bind (_returnvalue_roll _returnvalue_pitch _returnvalue_yaw) (`KismetMathLibrary.BreakRotator` (`self.K2_GetActorRotation`)))
  ;[1 1 1] Spin
  (`TimelineComponent.SetPlayRate` (`self.AxeAnimation`) (/ 1.0 (`self.AnimationTimer`)))
  (bind (_direction _axepitch) (`Timeline|AxeAnimation` :!via `PlayFromStart`)
    (:`Update`
      (`self.K2_SetActorRelativeRotation` (`KismetMathLibrary.MakeRotator` _returnvalue_roll _axepitch _returnvalue_yaw)))))

(fn `UserConstructionScript`
  (`parent.UserConstructionScript`))