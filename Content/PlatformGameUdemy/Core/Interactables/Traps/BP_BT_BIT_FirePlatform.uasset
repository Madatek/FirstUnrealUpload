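; Fire platform trap that, when the player interacts, shifts color as a warning, then burns with radius damage for one second.
; A timeline drives the dynamic material's TrapColor; on finishing, it sets the particle effect and enables Tick, which applies damage every frame.
; Reset clears the particles and reverses the same timeline, with IsInResetState distinguishing the pass.
; Once reset, it retriggers if an overlapping actor remains.
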(event `self.ReceiveTick`
  (params (DeltaSeconds :type "Float (single-precision)"))
  ;[1 1 1] When tick is enabled
  (`parent.ReceiveTick` DeltaSeconds)
  (`self.DoDamage` null (`self.RadiusOfDamage`)))

(event `self.ReceiveBeginPlay`
  ;[1 1 1] Spawn
  (`parent.ReceiveBeginPlay`)
  (bind _returnvalue (`PrimitiveComponent.CreateDynamicMaterialInstance` (`self.TrapMesh`) 0 null "None"))
  (set `self.MaterialInstanceReference` _returnvalue))

(event `self.PlayerInteracted`
  ;[1 1 1] Interaction and reset - enable and disable tick
  (if (not (`TimelineComponent.IsPlaying` (`self.PlatformColorAnimation`)))
    (bind (_direction _platformcolor) (`Timeline|PlatformColorAnimation` :!label _label)
      (:`Update`
        (`MaterialInstanceDynamic.SetVectorParameterValue` (`self.MaterialInstanceReference`) "TrapColor" _platformcolor))
      (:`Finished`
        (if (not (`self.bIsInResetState`))
          (`self.SetParticles` (`self.ParticleEffect`))
          (`self.SetActorTickEnabled` true)
          (`KismetSystemLibrary.Delay` 1.0)
          (`self.SetActorTickEnabled` false)
          (`self.Reset`)
          (set `self.bIsInResetState` true)
          (else
            (`/Engine/EditorBlueprintResources/StandardMacros.IsValid` (`self.OverlappingActor`)
              (:`Is Valid`
                (`self.PlayerInteracted`))
              (:`Is Not Valid`
                _))
            (set `self.bIsInResetState` false)))))))

(event `Reset`
  ;[1 1 1] Interaction and reset - enable and disable tick
  (`self.SetParticles` null)
  (goto _label :!via `Reverse`))

(fn `SetParticles`
  (params (NewParam :type "ParticleSystem Object Reference"))
  (`ParticleSystemComponent.SetTemplate` (`self.TrapEffect`) NewParam)
  (return))

(fn `UserConstructionScript`
  (`parent.UserConstructionScript`))