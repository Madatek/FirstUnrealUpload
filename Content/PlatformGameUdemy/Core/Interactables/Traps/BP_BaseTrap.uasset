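; BP_BaseTrap is the base Blueprint for traps in the platform game, providing a shared damage function with no active event logic of its own.
; DoDamage applies a fixed point damage to a given actor when it is valid, crediting the trap as causer.
; Otherwise it applies radial damage around the trap's location at the supplied radius, optionally drawing a debug sphere when DebugDamage is set.
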(fn `DoDamage`
  (params (ActorToDamage :type "Actor Object Reference") (DamageRadius :type "Float (double-precision)"))
  (bind _returnvalue (`self.K2_GetActorLocation`))
  (set `self.Damage Radius` DamageRadius)
  (bind _output_get (set `self.Actor to Damage` ActorToDamage))
  (`/Engine/EditorBlueprintResources/StandardMacros.IsValid` _output_get
    (:`Is Valid`
      (`GameplayStatics.ApplyDamage` (`self.Actor to Damage`) 100.0 null self)
      (return))
    (:`Is Not Valid`
      (`GameplayStatics.ApplyRadialDamage` :`BaseDamage` 100.0 :`Origin` _returnvalue :`DamageRadius` (`self.Damage Radius`) :`DamageCauser` self :`InstigatedByController` null)
      (if (`self.bDebugDamage`)
        (`KismetSystemLibrary.DrawDebugSphere` _returnvalue (`self.Damage Radius`) 12 (struct :`R` 1.0 :`G` 1.0 :`B` 1.0 :`A` 1.0) 0.5 0.2)
        (return)))))

(fn `UserConstructionScript`)