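; Base enemy character for a platformer that starts its AI controller on BeginPlay with its own blackboard and behavior tree.
; A top hit from the player bounces them and destroys the enemy if jumpable; other hits damage the player unless it is launched.
; Taking damage stops AI and physics-launches the enemy, which then damages non-player actors it overlaps and expires.
; A LookAt event rotates it toward a target.
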(event `self.ReceiveBeginPlay`
  (bind _asaic_base_enemy (cast `/Game/PlatformGameUdemy/Core/Characters/AI/General/AIC_BaseEnemy` (`self.GetController`)))
  (bind _output_get (set `self.MyAiController` _asaic_base_enemy))
  (`/Game/PlatformGameUdemy/Core/Characters/AI/General/AIC_BaseEnemy.InitializeAI` _output_get self (`self.AiBlackBoardData`) (`self.AiBehaviorTree`)))

(event `self.ReceiveHit`
  (params (MyComp :type "PrimitiveComponent Object Reference") (Other :type "Actor Object Reference") (OtherComp :type "PrimitiveComponent Object Reference") (bSelfMoved :type Boolean) (HitLocation :type "Vector Structure") (HitNormal :type "Vector Structure") (NormalImpulse :type "Vector Structure") (Hit :type "HitResult Structure (by ref)"))
  (`/Game/PlatformGameUdemy/Core/Utility/BPML_Utility.ActorIsPlayer` Other
    (:`IsPlayer`
      (if true
        (set `self.HitInstigator` Other)
        (if (and (`|EnumEquality` (`/Game/PlatformGameUdemy/Core/Utility/BP_FL_Utility.CheckHitSide` HitNormal 0.5) "NewEnumerator4") (`self.bCanBeJumped`))
          (`self.UpHit`)
          (else
            (`self.OtherSideHit`)))
        (set `self.HitInstigator` null)))))

(event `UpHit`
  (`KismetSystemLibrary.PrintString` "UpHit")
  (message `/Game/PlatformGameUdemy/Core/Interactables/Common/Bp_Interactables.Launch Actor` (`self.HitInstigator`) (0.0 0.0 600.0))
  (`self.K2_DestroyActor`))

(event `OtherSideHit`
  (`self.IsBeingLaunched`
    (:`else`
      (`KismetSystemLibrary.PrintString` "OtherHit")
      (`GameplayStatics.ApplyDamage` (`self.HitInstigator`) 100.0 null self))))

(event `self.ReceiveAnyDamage`
  (params (Damage :type "Float (single-precision)") (DamageType :type "DamageType Object Reference") (InstigatedBy :type "Controller Object Reference") (DamageCauser :type "Actor Object Reference"))
  (bind (_returnvalue_x _returnvalue_y) (`self.PrepareForceValue` DamageCauser))
  (bind _capsulecomponent (`self.CapsuleComponent`))
  (`/Game/PlatformGameUdemy/Core/Characters/AI/General/AIC_BaseEnemy.StopAI` (`self.MyAiController`))
  (`PrimitiveComponent.SetCollisionResponseToAllChannels` _capsulecomponent "ECR_Overlap")
  (`PrimitiveComponent.SetSimulatePhysics` _capsulecomponent true)
  (`PrimitiveComponent.AddForce` _capsulecomponent (`KismetMathLibrary.MakeVector` _returnvalue_x _returnvalue_y) "None" true)
  (set `self.bIsLaunched` true)
  (`self.SetLifeSpan` 5.0))

(event `self.ReceiveActorBeginOverlap`
  (params (OtherActor :type "Actor Object Reference"))
  (`/Game/PlatformGameUdemy/Core/Utility/BPML_Utility.ActorIsPlayer` OtherActor
    (:`IsNotPlayer`
      (`/Game/PlatformGameUdemy/Core/Utility/BPML_Utility.ActorNotItself` self OtherActor
        (:`IsNotSame`
          (`self.IsBeingLaunched`
            (:`true`
              (`GameplayStatics.ApplyDamage` OtherActor 1000.0 null self))))))))

(event `LookAt`
  (params (DeltaTime :type "Float (double-precision)"))
  (bind _lookattarget (`self.LookAtTarget`))
  (bind (_returnvalue_roll _returnvalue_yaw) (`self.SetUpValuesForRotation` _lookattarget))
  (set `self.Delta Time` DeltaTime)
  (if (`KismetSystemLibrary.IsValid` _lookattarget)
    (`self.K2_SetActorRotation` (`KismetMathLibrary.MakeRotator` _returnvalue_roll 0.0 _returnvalue_yaw))))

(fn `UserConstructionScript`
  (`SceneComponent.SetHiddenInGame` (`self.TextRender`) (not (`self.bDebugTextOn`)) false))