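; BP_BE_AreaEnemy is an area-attack enemy Blueprint that performs a spinning sword attack, triggered one second after BeginPlay.
; AttackAnimation zeroes the sword pivot's rotation, then plays the AttackRotation timeline, scaling its play rate by the inverse of AnimationTime.
; The timeline drives the actor's yaw each update and tilts the sword pivot 60 degrees when finished.
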(event `self.ReceiveBeginPlay`
  (`parent.ReceiveBeginPlay`)
  (`KismetSystemLibrary.Delay` 1.0)
  (`self.AttackAnimation`))

(event `AttackAnimation`
  (`SceneComponent.K2_SetRelativeRotation` :`self` (`self.ExampleSwordPivot`))
  (`TimelineComponent.SetPlayRate` (`self.AttackRotation`) (/ 1.0 (`self.AnimationTime`)))
  (bind (_direction _rotationrate) (`Timeline|AttackRotation`)
    (:`Update`
      (`self.K2_SetActorRotation` (`KismetMathLibrary.MakeRotator` 0.0 0.0 _rotationrate)))
    (:`Finished`
      (`SceneComponent.K2_SetRelativeRotation` (`self.ExampleSwordPivot`) (struct :`Roll` 60.0) false false))))

(fn `UserConstructionScript`
  (`parent.UserConstructionScript`))