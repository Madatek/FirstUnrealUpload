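; Patrolling enemy actor that holds a route of TargetPoint actors for an AI character in the platform game.
; GetNextPatrolPoint enables tick, advances the index with wraparound, and returns the next point as LookAtTarget.
; Underscore-prefixed helpers author the route by spawning points at the enemy's transform (refilling empty slots first), removing a chosen point, or clearing all.
; Tick only calls the parent; the LookAt call in the event graph is unconnected.
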(event `self.ReceiveTick`
  (params (DeltaSeconds :type "Float (single-precision)"))
  (`parent.ReceiveTick` DeltaSeconds))

(fn `_AddPatrolPoint`
  (bind _patrolpoints (`self.PatrolPoints`))
  (bind _returnvalue (`KismetArrayLibrary.Array_Find` _patrolpoints))
  (bind _returnvalue_2 (`|SpawnActorFromClass` "/Script/Engine.TargetPoint" (`self.GetTransform`) "Undefined" "OverrideRootScale" null null))
  (if (!= _returnvalue -1)
    (`KismetArrayLibrary.Array_Set` (`self.PatrolPoints`) _returnvalue _returnvalue_2)
    (else
      (`KismetArrayLibrary.Array_Add` _patrolpoints _returnvalue_2)))
  (return))

(fn `_ClearAllPath`
  (bind _patrolpoints (`self.PatrolPoints`))
  (for _array_element _patrolpoints
    (`self.K2_DestroyActor` _array_element))
  (`KismetArrayLibrary.Array_Clear` _patrolpoints)
  (return))

(fn `_RemovePatrolPoint`
  (bind _output (`|GetArrayItem` (`self.PatrolPoints`) (`self.PatrolPointToRemove`)))
  (if (`KismetArrayLibrary.Array_IsValidIndex` (`self.PatrolPoints`) (`self.PatrolPointToRemove`))
    (`/Engine/EditorBlueprintResources/StandardMacros.IsValid` _output
      (:`Is Valid`
        (`self.K2_DestroyActor` _output))
      (:`Is Not Valid`
        _))
    (`KismetArrayLibrary.Array_Remove` (`self.PatrolPoints`) (`self.PatrolPointToRemove`))
    (return)
    (else
      (return))))

(fn `GetNextPatrolPoint`
  (returns (CurrentPatrolPoint :type "Actor Object Reference"))
  (bind _returnvalue (+ (`self.PatrolPointIndex`) 1))
  (`self.SetActorTickEnabled` true)
  (bind _output_get (set `self.PatrolPointIndex` (select `bool` (`KismetArrayLibrary.Array_IsValidIndex` (`self.PatrolPoints`) _returnvalue) :`true` _returnvalue)))
  (bind _output_get_2 (set `self.LookAtTarget` (`|GetArrayItem` (`self.PatrolPoints`) _output_get)))
  (return _output_get_2))

(fn `UserConstructionScript`
  (`parent.UserConstructionScript`))