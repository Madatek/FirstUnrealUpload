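; Base player character for the platformer, handling protection levels, damage, invincibility, death and checkpoint registration at spawn.
; A CharacterState gates hits and pickups: hits lower protection and trigger blinking pawn-ignoring invincibility, while maxed protection can start invincibility that loops DoDamage.
; A dynamic material colors the protection marker, and a looping-timer macro drives timed states.
; Death ragdolls the mesh and notifies the game mode; attack and dodge inputs go out through dispatchers.
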(event `self.ReceiveAnyDamage`
  (params (Damage :type "Float (single-precision)") (DamageType :type "DamageType Object Reference") (InstigatedBy :type "Controller Object Reference") (DamageCauser :type "Actor Object Reference"))
  ;[1 1 1] Damage
  (if (`self.bIsDead`)
    _
    (elif (`DamageType.bCausedByWorld` DamageType)
      (`self.Death`)
      (else
        (`self.CheckCharacterState`
          (:`Normal`
            (`self.RemoveProtectionEvent`)))))))

(event `BeInvincible`
  ;[1 1 1] ProtectionAndInvincibility
  (set `self.CharacterState` "NewEnumerator2")
  (`self.LoopTimerManager` "DoDamage" 0.0 (`self.InvincibilityTime`)
    (:`TimerEnd`
      (`self.RemoveProtectionEvent`)
      (set `self.CharacterState` "NewEnumerator0"))))

(event `AddProtectionLevel`
  ;[1 1 1] ProtectionAndInvincibility
  (`self.CheckCharacterState`
    (:`Normal`
      _)
    (:`DamageInvincibility`
      _))
  (bind _currentprotectionlevel (`self.ProtectionLevelManager` true))
  (if (and (== _currentprotectionlevel (`self.ProtLevelToBeInvincible`)) (`self.CanBeInvincible`))
    (`self.BeInvincible`)))

(event `GetDamage`
  ;[1 1 1] Damage
  (set `self.CharacterState` "NewEnumerator1")
  (`self.CapsuleComponentCollisionManager` (`|MakeArray` "ECC_Pawn" :!type "ECollisionChannel Enum"))
  (`self.LoopTimerManager` "MeshBlink" 0.1 3.0
    (:`TimerEnd`
      (`SceneComponent.SetVisibility` (`self.Mesh`) true false)
      (`self.CapsuleComponentCollisionManager` (`|MakeArray` "ECC_Pawn" :!type "ECollisionChannel Enum") "ECR_Block")
      (set `self.CharacterState` "NewEnumerator0"))))

(event `MeleeAttack1Pressed`
  (params (bPressed :type Boolean))
  ;[1 1 1] Damage
  (`self.OnMeleeAttack1Pressed` bPressed))

(event `RemoveProtectionEvent`
  ;[1 1 1] ProtectionAndInvincibility
  (bind _currentprotectionlevel (`self.ProtectionLevelManager` false))
  (if (< _currentprotectionlevel 1)
    (`self.Death`)
    (set `self.CurrentProtectionLevel` 0)
    (else
      (`self.GetDamage`))))

(event `MeleeAttack1Released`
  ;[1 1 1] Damage
  (`self.OnMeleeAttack1Released`))

(event `Death`
  (bind _mesh (`self.Mesh`))
  ;[1 1 1] Death
  (set `self.bIsDead` true)
  (`self.CapsuleComponentCollisionManager` (`|MakeArray` "ECC_Pawn" "ECC_WorldDynamic" :!type "ECollisionChannel Enum"))
  (`/Game/PlatformGameUdemy/Core/Characters/Player/BP_PlatfromPlayerController.DisableController` (cast `/Game/PlatformGameUdemy/Core/Characters/Player/BP_PlatfromPlayerController` (`self.GetController`) :!pure true))
  (`PrimitiveComponent.SetCollisionProfileName` _mesh "Ragdoll" false)
  (`SkeletalMeshComponent.SetAllBodiesSimulatePhysics` _mesh true)
  (`self.CharacterUpdateMovementForDeath`)
  (`self.SendDeathSignalToGameMode`))

(event `self.ReceiveBeginPlay`
  ;[1 1 1] Miscellaneous
  (set `/Game/PlatformGameUdemy/Core/GameFramework/BP_PlatformGameMode.NextSpawnedClass` (`GameplayStatics.GetObjectClass` self) (cast `/Game/PlatformGameUdemy/Core/GameFramework/BP_PlatformGameMode` (`GameplayStatics.GetGameMode`) :!pure true))
  (set `self.bIsDead` false)
  (bind _returnvalue (`PrimitiveComponent.CreateDynamicMaterialInstance` (`self.ProtectionMarker`) 0 "/Game/PlatformGameUdemy/Core/Characters/Player/M_ProtectionMarker.M_ProtectionMarker" "None"))
  (set `self.ProtectionMarkerInstanceMaterial` _returnvalue)
  (set `self.My Controller` (`self.GetMyController`))
  (bind _output_get (set `self.GameModeReference` (cast `/Game/PlatformGameUdemy/Core/GameFramework/BP_PlatformGameMode` (`GameplayStatics.GetGameMode`) :!pure true)))
  (`/Game/PlatformGameUdemy/Core/GameFramework/BP_PlatformGameMode.RegisterNewCheckpoint` _output_get (`self.K2_GetActorLocation`))
  (`self.ProtectionMarkerGraphicUpdate`))

(event `MeshBlink`
  ;[1 1 1] Miscellaneous
  (bind _isa (`/Engine/EditorBlueprintResources/StandardMacros.FlipFlop`)
    (:`A`
      _)
    (:`B`
      _))
  (`SceneComponent.SetVisibility` (`self.Mesh`) _isa false))

(event `/Game/PlatformGameUdemy/Core/Interactables/Common/Bp_Interactables.Launch Actor`
  (params (LaunchSpeed :type "Vector Structure"))
  ;[1 1 1] Miscellaneous
  (`self.LaunchCharacter` LaunchSpeed))

(event `SendDeathSignalToGameMode`
  ;[1 1 1] Death
  (`KismetSystemLibrary.Delay` 1.5)
  (`/Game/PlatformGameUdemy/Core/GameFramework/BP_PlatformGameMode.PlayerDeath` (`self.GameModeReference`) (`self.GetMyController`))
  (`self.K2_DestroyActor`))

(event `HandleDodgeLeft`
  ;[1 1 1] Miscellaneous
  (`self.OnDodgeLeft`)
  (set `self.bInputDodgeLeftIsBeingPressed` true))

(event `HandleDodgeRight`
  ;[1 1 1] Miscellaneous
  (`self.OnDodgeRight`)
  (set `self.bInputDodgeLeftIsBeingPressed` true))

(event `ReleaseDodgeRight`
  ;[1 1 1] Miscellaneous
  (set `self.bInputDodgeRightIsBeingPressed` false))

(event `ReleaseDodgeLeft`
  ;[1 1 1] Miscellaneous
  (set `self.bInputDodgeLeftIsBeingPressed` false))

(fn `CapsuleComponentCollisionManager`
  (params (CollisionChannelsToModify :type "Array of ECollisionChannel Enum") (NewResponse :type "ECollisionResponse Enum" :default "ECR_Ignore"))
  (for _array_element CollisionChannelsToModify
    (`PrimitiveComponent.SetCollisionResponseToChannel` (`self.CapsuleComponent`) _array_element NewResponse))
  (return))

(fn `CharacterUpdateMovementForDeath`
  (bind _charactermovement (`self.CharacterMovement`))
  (`MovementComponent.SetPlaneConstraintAxisSetting` _charactermovement "Z")
  (`MovementComponent.SetPlaneConstraintEnabled` _charactermovement false)
  (`MovementComponent.StopMovementImmediately` _charactermovement)
  (return))

(fn `GetMyController`
  (returns (MyController :type "/Game/PlatformGameUdemy/Core/Characters/Player/BP_PlatfromPlayerController Object Reference"))
  (return (cast `/Game/PlatformGameUdemy/Core/Characters/Player/BP_PlatfromPlayerController` (`self.GetController`) :!pure true)))

(fn `ProtectionLevelManager`
  (params (Add :type Boolean))
  (returns (CurrentProtectionLevel :type Integer))
  (bind _currentprotectionlevel (`self.CurrentProtectionLevel`))
  (if Add
    (if (< (`self.CurrentProtectionLevel`) (`self.ProtLevelToBeInvincible`))
      (`/Engine/EditorBlueprintResources/StandardMacros.IncrementInt` _currentprotectionlevel
        (:`  `
          (`self.ProtectionMarkerGraphicUpdate` :!label _label)
          (return (`self.CurrentProtectionLevel`)))))
    (else
      (`/Engine/EditorBlueprintResources/StandardMacros.DecrementInt` _currentprotectionlevel
        (:`  `
          (goto _label))))))

(fn `ProtectionMarkerGraphicUpdate`
  (`MaterialInstanceDynamic.SetVectorParameterValue` (`self.ProtectionMarkerInstanceMaterial`) "MarkerColor" (select `int` (`self.CurrentProtectionLevel`) :`0` (struct :`R` 1.0 :`G` 1.0 :`B` 1.0 :`A` 1.0) :`1` (struct :`R` 0.040045 :`G` 1.0 :`A` 1.0) :`2` (struct :`R` 0.017893 :`B` 1.0 :`A` 1.0) :`3` (struct :`R` 1.0 :`G` 0.975086 :`A` 1.0) :`4` (struct :`R` 1.0 :`A` 1.0) :!type "LinearColor Structure"))
  (return))

(fn `UserConstructionScript`
  (if (`self.bShowDamageArea`)
    (`KismetSystemLibrary.FlushPersistentDebugLines`)
    (`KismetSystemLibrary.DrawDebugSphere` (`self.K2_GetActorLocation`) (`self.Damage Radius`) 12 (struct :`R` 1.0 :`G` 1.0 :`B` 1.0 :`A` 1.0) 5.0)
    (else
      (`KismetSystemLibrary.FlushPersistentDebugLines`))))