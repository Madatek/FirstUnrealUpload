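; Player controller for the platformer that turns input into actions on the possessed pawn, with game-only input and a hidden cursor.
; Movement follows control yaw, and look axes feed pitch and yaw.
; Jump either launches BP_BasePlayer upward once when CanBeLaunched is set or performs a normal jump, while Tornado press and release forward to HandleTornado.
; Custom events handle pawn swapping by toggling input around UnPossess and Possess.
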(event `self.ReceiveBeginPlay`
  (`WidgetBlueprintLibrary.SetInputMode_GameOnly` self)
  (set `self.bShowMouseCursor` false))

(event `InputAction|Jump`
  (params (Key :type "Key Structure"))
  (bind _as_character (`self.As Character`))
  (:`Pressed`
    (bind _asbp_base_player (cast `/Game/PlatformGameUdemy/Core/Characters/Player/BP_BasePlayer` (`self.As Character`)))
    (set `self.As BP Base Player` _asbp_base_player)
    (if (`/Game/PlatformGameUdemy/Core/Characters/Player/BP_BasePlayer.CanBeLaunched` (`self.As BP Base Player`))
      (`Character.LaunchCharacter` (`self.As BP Base Player`) (0.0 0.0 700.0) false false)
      (set `/Game/PlatformGameUdemy/Core/Characters/Player/BP_BasePlayer.CanBeLaunched` false (`self.As BP Base Player`))
      (else
        (`/Engine/EditorBlueprintResources/StandardMacros.IsValid` _as_character
          (:`Is Valid`
            (`Character.Jump` _as_character))))))
  (:`Released`
    (set `self.As Character` (cast `Character` (`self.K2_GetPawn`) :!pure true))
    (`/Engine/EditorBlueprintResources/StandardMacros.IsValid` (`self.As Character`)
      (:`Is Valid`
        (`Character.StopJumping` (`self.As Character`))))))

(event `InputAxis|MoveForward`
  (params (AxisValue :type "Float (single-precision)"))
  (bind _returnvalue (`self.K2_GetPawn`))
  (bind (_returnvalue_roll _returnvalue_pitch _returnvalue_yaw) (`KismetMathLibrary.BreakRotator` (`Pawn.GetControlRotation` _returnvalue)))
  (`Pawn.AddMovementInput` _returnvalue (`KismetMathLibrary.GetForwardVector` (`KismetMathLibrary.MakeRotator` 0.0 0.0 _returnvalue_yaw)) AxisValue false))

(event `RemoveFromPlayer`
  (`self.DisableController`)
  (`self.UnPossess`))

(event `InputAxis|MoveRight`
  (params (AxisValue :type "Float (single-precision)"))
  (bind _returnvalue (`self.K2_GetPawn`))
  (bind (_returnvalue_roll _returnvalue_pitch _returnvalue_yaw) (`KismetMathLibrary.BreakRotator` (`Pawn.GetControlRotation` _returnvalue)))
  (`Pawn.AddMovementInput` _returnvalue (`KismetMathLibrary.GetRightVector` (`KismetMathLibrary.MakeRotator` 0.0 0.0 _returnvalue_yaw)) AxisValue false))

(event `AssignNewPlayer`
  (params (PlayerToAssign :type "Pawn Object Reference"))
  (`self.Possess` PlayerToAssign)
  (`self.EnableInput` self))

(event `InputAxis|LookUp`
  (params (AxisValue :type "Float (single-precision)"))
  (`Pawn.AddControllerPitchInput` (`self.K2_GetPawn`) AxisValue))

(event `InputAction|Tornado`
  (params (Key :type "Key Structure"))
  (bind _asbp_base_player (cast `/Game/PlatformGameUdemy/Core/Characters/Player/BP_BasePlayer` (`self.K2_GetPawn`) :!pure true))
  (:`Pressed`
    (`/Game/PlatformGameUdemy/Core/Characters/Player/BP_BasePlayer.HandleTornado` _asbp_base_player true))
  (:`Released`
    (`/Game/PlatformGameUdemy/Core/Characters/Player/BP_BasePlayer.HandleTornado` _asbp_base_player false)))

(event `DisableController`
  (`self.DisableInput` self))

(event `InputAxis|Turn`
  (params (AxisValue :type "Float (single-precision)"))
  (`Pawn.AddControllerYawInput` (`self.K2_GetPawn`) AxisValue))

(fn `DummyTornadoFunction`
  (params (bPressed :type Boolean)))

(fn `UserConstructionScript`)