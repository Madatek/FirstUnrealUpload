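; Blueprint function library of shared helpers for the platform game.
; It fetches the game mode cast to BP_PlatformGameMode with a success flag, and writes the next level name and last-level flag onto it.
; CheckHitSide classifies a normalized hit vector into one of six sides by testing X, Y, then Z against a clamped threshold, printing each result and falling back to the Down value with a warning.
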(fn `CheckHitSide`
  (params (NormalizedHit :type "Vector Structure") (CheckOffset :type "Float (double-precision)"))
  (returns (HitSide :type "/Game/PlatformGameUdemy/Core/Interactables/Common/EHitSide Enum"))
  (bind _x (.x NormalizedHit))
  (bind _y (.y NormalizedHit))
  (bind _z (.z NormalizedHit))
  (bind _returnvalue (`KismetMathLibrary.FClamp` CheckOffset))
  (bind _returnvalue_2 (* _returnvalue -1.0))
  (if (> _x _returnvalue)
    (`KismetSystemLibrary.PrintString` null "Front")
    (return "NewEnumerator0")
    (elif (< _x _returnvalue_2)
      (`KismetSystemLibrary.PrintString` null "BAck")
      (return "NewEnumerator1")
      (elif (> _y _returnvalue)
        (`KismetSystemLibrary.PrintString` null "Left")
        (return "NewEnumerator2")
        (elif (< _y _returnvalue_2)
          (`KismetSystemLibrary.PrintString` null "Right")
          (return "NewEnumerator3")
          (elif (> _z _returnvalue)
            (`KismetSystemLibrary.PrintString` null "Down")
            (return "NewEnumerator5")
            (elif (< _z _returnvalue_2)
              (`KismetSystemLibrary.PrintString` null "up")
              (return "NewEnumerator4")
              (else
                (`KismetSystemLibrary.PrintString` null "WARNING: CAN'T DETERMINE HIT SIDE")
                (return "NewEnumerator5")))))))))

(fn `GetPlatformGameMode`
  (params (WorldContextObject :type "Object Object Reference"))
  (returns (`AsBP Platform Game Mode` :type "/Game/PlatformGameUdemy/Core/GameFramework/BP_PlatformGameMode Object Reference") (bSuccess :type Boolean))
  (bind _asbp_platform_game_mode (cast `/Game/PlatformGameUdemy/Core/GameFramework/BP_PlatformGameMode` (`GameplayStatics.GetGameMode` WorldContextObject))
    (:`then`
      (return _asbp_platform_game_mode true))
    (:`CastFailed`
      (return null false))))

(fn `SetNextLevelName`
  (params (NextLevelInput :type String) (bIsLastLevel :type Boolean))
  (bind _asbp_platform_game_mode (cast `/Game/PlatformGameUdemy/Core/GameFramework/BP_PlatformGameMode` (`GameplayStatics.GetGameMode` null)))
  (set `/Game/PlatformGameUdemy/Core/GameFramework/BP_PlatformGameMode.NextLevelName` NextLevelInput _asbp_platform_game_mode)
  (set `/Game/PlatformGameUdemy/Core/GameFramework/BP_PlatformGameMode.bIsLastLevel` bIsLastLevel _asbp_platform_game_mode)
  (return))