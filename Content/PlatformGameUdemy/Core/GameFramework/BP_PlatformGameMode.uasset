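; Platformer game mode that runs level rules for collectibles, lives, box breaking, checkpoints and win or lose screens.
; It seeds lives, credits and swap tokens from GI_PlatformGameInstance, notifies it of some changes, and broadcasts counters through a data-update dispatcher.
; Points convert to extra lives at a threshold, and death respawns the player at the last checkpoint with a fade sequence.
; Character swapping, optionally token-gated, replaces the pawn in place, alternating BigVegas and GreenDragon.
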(event `FailSwapPlayer`
  (`KismetSystemLibrary.PrintString` "No Swap Tokens Available"))

(event `SwapPlayer`
  (params (IsUsingCharToken :type Boolean))
  (if IsUsingCharToken
    (if (> (`self.ChangeCharTokens`) 0)
      (`/Engine/EditorBlueprintResources/StandardMacros.DecrementInt` (`self.ChangeCharTokens`)
        (:`  `
          (`self.UpdateData`)
          (`self.CommitChangePlayer` :!label _label)))
      (else
        (`self.FailSwapPlayer`)))
    (else
      (goto _label))))

(event `self.ReceiveBeginPlay`
  ;[1 1 1] BeginPlay - triggers on level spawn
  (bind _asgi_platform_game_instance (cast `/Game/PlatformGameUdemy/Core/GameFramework/GI_PlatformGameInstance` (`GameplayStatics.GetGameInstance`)))
  (set `self.LifeCounter` (`/Game/PlatformGameUdemy/Core/GameFramework/GI_PlatformGameInstance.Lives` _asgi_platform_game_instance))
  (bind _returnvalue (`|CreateWidget` "/Game/PlatformGameUdemy/Core/UI/WBP_PlayerStatistics.WBP_PlayerStatistics_C"))
  (set `self.Credits` (`/Game/PlatformGameUdemy/Core/GameFramework/GI_PlatformGameInstance.Credits` _asgi_platform_game_instance))
  (set `self.ChangeCharTokens` (`/Game/PlatformGameUdemy/Core/GameFramework/GI_PlatformGameInstance.CharSwapTokens` _asgi_platform_game_instance))
  (`UserWidget.AddToViewport` _returnvalue 0)
  (`self.UpdateData`))

(event `UpdateData`
  ;[1 1 1] DataUpdate for Widget
  (`self.OnDataUpdate` (`self.PointsCounter`) (`self.LifeCounter`) (`self.BrokenBoxes`) (`self.BoxTotal`) (`self.Credits`) (`self.ChangeCharTokens`)))

(event `AddCollectable`
  (params (TypeOfCollectable :type "/Game/PlatformGameUdemy/Core/Interactables/Collectables/ECollectableType Enum" :default "NewEnumerator0"))
  ;[1 1 1] Collectibles
  (switch `/Game/PlatformGameUdemy/Core/Interactables/Collectables/ECollectableType` TypeOfCollectable
    (:`NewEnumerator0`
      (`self.AddPoint`)
      (`self.UpdateData` :!label _label_2))
    (:`NewEnumerator1`
      (`self.AddLife`)
      (goto _label_2))
    (:`NewEnumerator2`
      (`self.OnTargetCollected`))
    (:`NewEnumerator3`
      (`self.AddChangeCharToken`)
      (goto _label_2))))

(event `AddPoint`
  ;[1 1 1] Collectibles
  (bind (_tresholdreached _stringtoprint) (`self.PointCounter` (`self.PointToLife`))
    (:`  `
      (`KismetSystemLibrary.PrintString` _stringtoprint)
      (if _tresholdreached
        (`self.AddLife`)
        (set `self.PointsCounter` 0)))))

(event `WinGame`
  ;[1 1 1] WinGame, on winning platform primed and activated
  (`self.ShowGameOverScreen` true))

(event `PlayerDeath`
  (params (DeadPlayerController :type "/Game/PlatformGameUdemy/Core/Characters/Player/BP_PlatfromPlayerController Object Reference"))
  ;[1 1 1] Death related
  (set `self.Dead Player Controller` DeadPlayerController)
  (bind _result (`/Engine/EditorBlueprintResources/StandardMacros.DecrementInt` (`self.LifeCounter`))
    (:`  `
      (if (< _result 0)
        (`self.LoseGame`)
        (else
          (`self.UpdateData`)
          (bind (_outactor _returnvalue) (`LevelSequencePlayer.CreateLevelSequencePlayer` "/Game/PlatformGameUdemy/Core/GameFramework/LS_DeathFade.LS_DeathFade"))
          (`MovieSceneSequencePlayer.Play` _returnvalue)
          (`/Game/PlatformGameUdemy/Core/Characters/Player/BP_PlatfromPlayerController.RemoveFromPlayer` (`self.Dead Player Controller`))
          (bind _returnvalue_2 (`|SpawnActorFromClass` (`self.NextSpawnedClass`) (`KismetMathLibrary.MakeTransform` (`self.CurrentCheckpointPosition`)) "Undefined" "OverrideRootScale" null null))
          (`/Game/PlatformGameUdemy/Core/Characters/Player/BP_PlatfromPlayerController.AssignNewPlayer` (`self.Dead Player Controller`) (cast `Pawn` _returnvalue_2 :!pure true))
          (`/Game/PlatformGameUdemy/Core/GameFramework/GI_PlatformGameInstance.LivesUpdate` (cast `/Game/PlatformGameUdemy/Core/GameFramework/GI_PlatformGameInstance` (`GameplayStatics.GetGameInstance`) :!pure true)))))))

(event `AddLife`
  ;[1 1 1] Collectibles
  (bind _result (`/Engine/EditorBlueprintResources/StandardMacros.IncrementInt` (`self.LifeCounter`))
    (:`  `
      (`KismetSystemLibrary.PrintString` (`KismetStringLibrary.Conv_IntToString` _result))
      (bind _asgi_platform_game_instance (cast `/Game/PlatformGameUdemy/Core/GameFramework/GI_PlatformGameInstance` (`GameplayStatics.GetGameInstance`)))
      (`/Game/PlatformGameUdemy/Core/GameFramework/GI_PlatformGameInstance.LivesUpdate` _asgi_platform_game_instance))))

(event `LoseGame`
  ;[1 1 1] Death related
  (`self.ShowGameOverScreen` false))

(event `AddChangeCharToken`
  ;[1 1 1] Collectibles
  (bind _result (`/Engine/EditorBlueprintResources/StandardMacros.IncrementInt` (`self.ChangeCharTokens`))
    (:`  `
      (`KismetSystemLibrary.PrintString` (`KismetStringLibrary.Conv_IntToString` _result))
      (bind _asgi_platform_game_instance (cast `/Game/PlatformGameUdemy/Core/GameFramework/GI_PlatformGameInstance` (`GameplayStatics.GetGameInstance`)))
      (`/Game/PlatformGameUdemy/Core/GameFramework/GI_PlatformGameInstance.ChangeCharTokenUpdate` _asgi_platform_game_instance))))

(event `BoxBroken`
  ;[1 1 1] Box breaking related
  (bind _result (`/Engine/EditorBlueprintResources/StandardMacros.IncrementInt` (`self.BrokenBoxes`))
    (:`  `
      (`self.UpdateData`)
      (if (== _result (`self.BoxTotal`))
        (`self.OnAllBoxDestroyed`)))))

(event `RegisterNewCheckpoint`
  (params (NewCheckPointPosition :type "Vector Structure"))
  ;[1 1 1] Checkpoint
  (if (not (== NewCheckPointPosition (`self.CurrentCheckpointPosition`)))
    (bind _output_get (set `self.CurrentCheckpointPosition` NewCheckPointPosition))
    (`KismetSystemLibrary.PrintString` (`KismetStringLibrary.Conv_VectorToString` _output_get))))

(event `IncrementBoxTotal`
  ;[1 1 1] Box breaking related
  (`/Engine/EditorBlueprintResources/StandardMacros.IncrementInt` (`self.BoxTotal`)))

(fn `CommitChangePlayer`
  (bind _output_get (set `self.BPPlayerController` (cast `/Game/PlatformGameUdemy/Core/Characters/Player/BP_PlatfromPlayerController` (`GameplayStatics.GetPlayerController` 0) :!pure true)))
  (bind _output_get_2 (set `self.CurrentPawn` (`Controller.K2_GetPawn` _output_get)))
  (set `self.OldPawnLocation` (`self.K2_GetActorLocation` _output_get_2))
  (`/Game/PlatformGameUdemy/Core/Characters/Player/BP_PlatfromPlayerController.RemoveFromPlayer` (`self.BPPlayerController`))
  (`self.K2_DestroyActor` (`self.CurrentPawn`))
  (if (== (`GameplayStatics.GetObjectClass` (`self.CurrentPawn`)) "/Game/PlatformGameUdemy/Characters/Player/BP_BP_BigVegas.BP_BP_BigVegas_C")
    (set `self.NextSpawnedClass` "/Game/PlatformGameUdemy/Characters/Player/BP_BP_GreenDragon.BP_BP_GreenDragon_C")
    (else
      (set `self.NextSpawnedClass` "/Game/PlatformGameUdemy/Characters/Player/BP_BP_BigVegas.BP_BP_BigVegas_C")))
  (bind _returnvalue (`|SpawnActorFromClass` (`self.NextSpawnedClass`) (`KismetMathLibrary.MakeTransform` (`self.OldPawnLocation`)) "Undefined" "OverrideRootScale" null null))
  (`/Game/PlatformGameUdemy/Core/Characters/Player/BP_PlatfromPlayerController.AssignNewPlayer` (`self.BPPlayerController`) (cast `/Game/PlatformGameUdemy/Core/Characters/Player/BP_BasePlayer` _returnvalue :!pure true)))

(fn `ShowGameOverScreen`
  (params (bWin :type Boolean))
  (bind _returnvalue (`GameplayStatics.GetPlayerController` 0))
  (bind _returnvalue_2 (`|CreateWidget` "/Game/PlatformGameUdemy/Core/UI/WBP_GameOverScreen.WBP_GameOverScreen_C" null bWin (`self.BrokenBoxes`) (`self.BoxTotal`))) ; to replace with correct game over widget
  (`UserWidget.AddToViewport` _returnvalue_2 0)
  (`GameplayStatics.SetGamePaused` true)
  (`WidgetBlueprintLibrary.SetInputMode_UIOnlyEx` _returnvalue _returnvalue_2)
  (set `PlayerController.bShowMouseCursor` true _returnvalue)
  (return))

(fn `UserConstructionScript`)