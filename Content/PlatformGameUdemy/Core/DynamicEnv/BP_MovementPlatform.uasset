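; Moving platform actor that carries its pivot along a spline track at constant velocity, starting on BeginPlay.
; A timeline, with play rate set from TimeToCompleteMovement, drives the pivot's spline position, forward or reversed per IsReversed.
; ClosedLoop closes the spline and loops the timeline; otherwise finishing triggers a FlipFlop ping-pong between directions.
; The construction script previews the pivot's position at DebugTime.
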(event `self.ReceiveBeginPlay`
  (`TimelineComponent.SetPlayRate` (`self.PlatformMovementTimeline`) (/ 1.0 (`self.TimeToCompleteMovement`)))
  (`TimelineComponent.SetLooping` (`self.PlatformMovementTimeline`) (`self.bClosedLoop`))
  (`self.StartMovement`))

(event `StartMovement`
  (`self.IsReversedCheck`
    (:`IsReversed`
      (bind (_direction _time) (`Timeline|PlatformMovementTimeline` :!via `ReverseFromEnd` :!label _label)
        (:`Update`
          (`SceneComponent.K2_SetRelativeLocation` (`self.PlatformPivot`) (`SplineComponent.GetLocationAtTime` (`self.PlatformMovementTrack`) _time "Local" true) false false))
        (:`Finished`
          (`self.PingPong`))))
    (:`IsNotReversed`
      (goto _label))))

(event `PingPong`
  (`self.IsReversedCheck`
    (:`IsReversed`
      (`/Engine/EditorBlueprintResources/StandardMacros.FlipFlop`
        (:`A`
          (goto _label))
        (:`B`
          (goto _label :!via `ReverseFromEnd`))))
    (:`IsNotReversed`
      (`/Engine/EditorBlueprintResources/StandardMacros.FlipFlop`
        (:`A`
          (goto _label :!via `ReverseFromEnd`))
        (:`B`
          (goto _label))))))

(fn `UserConstructionScript`
  (`SplineComponent.SetClosedLoop` (`self.PlatformMovementTrack`) (`self.bClosedLoop`) true)
  (`SceneComponent.K2_SetRelativeLocation` (`self.PlatformPivot`) (`SplineComponent.GetLocationAtTime` (`self.PlatformMovementTrack`) (`self.DebugTime`) "Local" true) false false))